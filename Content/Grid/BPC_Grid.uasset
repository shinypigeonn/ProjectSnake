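; BPC_Grid is a grid Blueprint that converts a location into a snapped position on a flat square grid.
; GetGridLocation rounds X and Y to the nearest multiple of GridSize offset by half a cell, landing on cell centers if lines fall on multiples of GridSize.
; The returned Z is always zero, and the event graph holds only disabled placeholder events.
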(event EventBeginPlay)

(event EventTick
  (params (DeltaSeconds :type Float%20%28single-precision%29)))

(fn GetGridLocation
  (params (Location :type Vector))
  (bind _grid_size (Variables|Default|GetGrid_Size))
  (bind _grid_size_2 (Variables|Default|GetGrid_Size))
  (bind _grid_size_3 (Variables|Default|GetGrid_Size))
  (bind _returnvalue (/ _grid_size 2.0))
  (bind _returnvalue_2 (/ _grid_size_3 2.0))
  (return (Math|Vector|MakeVector (+ (* (Math|Conversions|ToFloat(Integer) (Math|Float|Round (/ (- (.x Location) _returnvalue) _grid_size_2))) _grid_size_3) _returnvalue_2) (+ (* (Math|Conversions|ToFloat(Integer) (Math|Float|Round (/ (- (.y Location) _returnvalue) _grid_size_2))) _grid_size_3) _returnvalue_2) 0.0)))